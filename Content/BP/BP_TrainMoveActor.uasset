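; Actor that drives a DoctorYellow train actor along the spline of a BP_RailSplineActor.
; Tick advances a distance by Speed, clamped to the spline length, and sets the train's location 150 units sideways from the tangent, with spline rotation plus a yaw offset.
; W nudges the train in Y; Space toggles IsStopTrain, which the live Tick ignores.
; Looping and circular-orbit movement remain as unconnected logic.
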(event EventBeginPlay
  (bind _railsplineactor (Variables|Default|GetRailSplineActor))
  (Input|EnableInput (Game|GetPlayerController 0))
  (Variables|Default|SetCurrentAngle 9e+01) ; 初期化
  (Utilities|IsValid _railsplineactor
    (:Is%20Valid
      (Variables|Default|SetLength (Spline|GetSplineLength (Variables|/Game/BP/BP_RailSplineActor.BP_RailSplineActor_C|GetSplineComponent _railsplineactor))))
    (:Is%20Not%20Valid
      (bind _outactors (Actor|GetAllActorsOfClass "/Game/BP/BP_RailSplineActor.BP_RailSplineActor_C"))
      (Variables|Default|SetLength (Spline|GetSplineLength (Variables|/Game/BP/BP_RailSplineActor.BP_RailSplineActor_C|GetSplineComponent (Utilities|Array|Get(acopy) _outactors)))))))

(event EventTick
  (params (DeltaSeconds :type Float%20%28single-precision%29))
  (bind _railsplineactor (Variables|Default|GetRailSplineActor))
  (bind _doctoryellow (Variables|Default|GetDoctorYellow))
  (bind _splinecomponent (Variables|/Game/BP/BP_RailSplineActor.BP_RailSplineActor_C|GetSplineComponent _railsplineactor))
  (bind _output_get (Variables|Default|SetDistance (Math|Float|Clamp(Float) (+ (Variables|Default|GetDistance) (* DeltaSeconds (Variables|Default|GetSpeed))) 0.0 (Variables|Default|GetLength))))
  (Transformation|SetActorLocation _doctoryellow (+ (Spline|GetLocationatDistanceAlongSpline _splinecomponent _output_get "World") (* (Math|Vector|CrossProduct (Math|Vector|Normalize (Spline|GetTangentatDistanceAlongSpline _splinecomponent _output_get "World")) "0.000000,0.000000,1.000000") -150)) false false)
  (Transformation|SetActorRotation _doctoryellow (Math|Rotator|MakeRotator (.Roll (Math|Rotator|BreakRotator (Spline|GetRotationatDistanceAlongSpline _splinecomponent _output_get "World"))) (.Pitch (Math|Rotator|BreakRotator (Spline|GetRotationatDistanceAlongSpline _splinecomponent _output_get "World"))) (+ (.Yaw (Math|Rotator|BreakRotator (Spline|GetRotationatDistanceAlongSpline _splinecomponent _output_get "World"))) (Variables|Default|GetYawOffset)))))

(event Input|KeyboardEvents|SpaceBar
  (params (Key :type Key%20Structure :default "None"))
  (:Pressed
    (if (Variables|Default|GetisStopTrain)
      (Variables|Default|SetisStopTrain false)
      (else
        (Variables|Default|SetisStopTrain true)))))

(event Input|KeyboardEvents|W
  (params (Key :type Key%20Structure :default "None"))
  (bind _doctoryellow (Variables|Default|GetDoctorYellow))
  (bind _returnvalue (Transformation|GetActorLocation _doctoryellow))
  (:Pressed
    (Transformation|SetActorLocation _doctoryellow (Math|Vector|MakeVector (.x _returnvalue) (+ (.y _returnvalue) (Variables|Default|GetMovementAmount)) (.z _returnvalue)) false false)))

(fn ConstructionScript)