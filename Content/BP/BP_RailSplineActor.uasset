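; BP_RailSplineActor is a spline-driven actor that lays railway track along an editable path.
; The construction script aligns the spline to the root transform, then adds one attached spline mesh component per segment using SM_railway_road.
; Each mesh bends between neighboring spline points using their local positions and tangents.
; The event graph holds only disabled placeholder events, so the actor has no runtime logic.
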(event EventBeginPlay)

(event Collision|EventActorBeginOverlap
  (params (OtherActor :type Actor%20Object%20Reference)))

(event EventTick
  (params (DeltaSeconds :type Float%20%28single-precision%29)))

(fn ConstructionScript
  (bind _splinecomponent (Variables|Default|GetSplineComponent))
  (bind _splinecomponent_2 (Variables|Default|GetSplineComponent))
  (Transformation|SetWorldTransform _splinecomponent (Transformation|GetWorldTransform (Variables|Default|GetDefaultSceneRoot)) false false)
  (for _index (range 0 (- (Class|SplineComponent|GetNumberOfSplineSegments _splinecomponent) 1)) ; 各セグメントごとに線路を生成
    (bind _returnvalue (AddComponent|AddSplineMeshComponent false))
    (Transformation|AttachComponentToComponent _returnvalue (Variables|Default|GetSplineComponent) "None" "KeepRelative" "KeepRelative" "KeepRelative" true)
    (Components|StaticMesh|SetStaticMesh _returnvalue "/Game/Train_pack/Skeletons/railway_road/SM_railway_road.SM_railway_road") ; 線路メッシュの割り当て
    (SplineMesh|SetStartandEnd _returnvalue (.Location (Spline|GetLocationandTangentatSplinePoint _splinecomponent_2 _index "Local")) (.Tangent (Spline|GetLocationandTangentatSplinePoint _splinecomponent_2 _index "Local")) (.Location (Spline|GetLocationandTangentatSplinePoint _splinecomponent_2 (+ _index 1) "Local")) (.Tangent (Spline|GetLocationandTangentatSplinePoint _splinecomponent_2 (+ _index 1) "Local")) true :!class /Script/Engine.SplineMeshComponent)))